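; BP_Ennemi2 is an enemy that chases the player on sight and, on overlap with its kill trigger, shows the death widget and pauses the game.
; PawnSensing sets CanSeePlayer and starts AIMoveTo, with a DoOnce starting chase audio.
; Tick fades the audio and resets the DoOnce while CanSeePlayer is false.
; The retriggerable delay after sighting sets CanSeePlayer true again, so nothing here clears it.
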(event OnComponentBeginOverlap(TouchThatYourDead)
  (params (OverlappedComponent :type Primitive%20Component%20Object%20Reference) (OtherActor :type Actor%20Object%20Reference) (OtherComp :type Primitive%20Component%20Object%20Reference) (OtherBodyIndex :type Integer) (bFromSweep :type Boolean) (SweepResult :type Hit%20Result%20Structure%20%28by%20ref%29))
  (Utilities|Casting|CastToBP_Player OtherActor)
  (bind _returnvalue (UserInterface|CreateWidget "/Game/Blueprint/UI/WBP_Death.WBP_Death_C"))
  (UserInterface|Viewport|AddtoViewport _returnvalue 0)
  (Game|SetGamePaused true))

(event OnSeePawn(PawnSensing)
  (params (Pawn :type Pawn%20Object%20Reference))
  (bind _asbp_player (Utilities|Casting|CastToBP_Player Pawn))
  (Utilities|FlowControl|Sequence
    (:then_0
      (Variables|Default|SetCanSeePlayer? true)
      (AI|AIMoveTo self "0, 0, 0" _asbp_player 5.0 false
        (:then
          (Utilities|FlowControl|DoOnce false
            (:Completed
              (Audio|Components|Audio|Play (Variables|Default|GetAudio) 0.0))))))
    (:then_1
      (Utilities|FlowControl|RetriggerableDelay 0.6)
      (Variables|Default|SetCanSeePlayer? true))))

(event EventBeginPlay
  ;[1 1 1] Create audio reference
  (bind _returnvalue (AddComponent|AddAudioComponent false))
  (Audio|Components|Audio|Stop _returnvalue)
  (Variables|Default|SetAudio _returnvalue))

(event EventTick
  (params (DeltaSeconds :type Float%20%28single-precision%29))
  (if (not (Variables|Default|GetCanSeePlayer?))
    (Utilities|FlowControl|Delay 0.2)
    (if (not (Variables|Default|GetCanSeePlayer?))
      (Audio|Components|Audio|FadeOut (Variables|Default|GetAudio) 5.0 0.0 "Linear" :!class /Script/Engine.AudioComponent)
      (Utilities|FlowControl|DoOnce false) ; enters at Reset
    )))

(fn ConstructionScript)