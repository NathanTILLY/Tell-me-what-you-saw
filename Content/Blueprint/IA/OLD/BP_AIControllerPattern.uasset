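; AI controller that drives a patrol-like pattern by cycling a Blackboard target through four vector positions.
; On BeginPlay it initializes the pattern Blackboard and runs the pattern Behavior Tree.
; An endless latent loop then writes each position in turn to the "MyEnnemi" key, separated by alternating short and long delays, so the timing is fixed rather than based on arrival or perception.
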(event EventBeginPlay
  (bind _blackboardcomponent (Class|AIController|UseBlackboard "/Game/Blueprint/IA/OLD/BB_AIBlackBoardPattern.BB_AIBlackBoardPattern"))
  (Variables|Default|SetBlackboard%20Component _blackboardcomponent)
  (AI|RunBehaviorTree "/Game/Blueprint/IA/OLD/BT_AIPatternBT.BT_AIPatternBT")
  (AI|Components|Blackboard|SetValueasVector (Variables|Default|GetBlackboard%20Component) (Utilities|Name|MakeLiteralName "MyEnnemi") (Variables|Default|GetVector2) :!label _label)
  (Utilities|FlowControl|Delay 3.0)
  (AI|Components|Blackboard|SetValueasVector (Variables|Default|GetBlackboard%20Component) (Utilities|Name|MakeLiteralName "MyEnnemi") (Variables|Default|GetVector3))
  (Utilities|FlowControl|Delay 6.0)
  (AI|Components|Blackboard|SetValueasVector (Variables|Default|GetBlackboard%20Component) (Utilities|Name|MakeLiteralName "MyEnnemi") (Variables|Default|GetVector4))
  (Utilities|FlowControl|Delay 3.0)
  (AI|Components|Blackboard|SetValueasVector (Variables|Default|GetBlackboard%20Component) (Utilities|Name|MakeLiteralName "MyEnnemi") (Variables|Default|GetVector1))
  (Utilities|FlowControl|Delay 6.0)
  (goto _label))

(fn ConstructionScript)