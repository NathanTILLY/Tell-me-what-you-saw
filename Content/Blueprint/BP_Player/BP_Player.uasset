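; First-person player character Blueprint handling movement, invertible look, sprint, crouch, flashlight and a pausing Escape menu.
; Sprint toggles speed caps that vary with the controller's medication flag, looping HP drain while running and regeneration otherwise.
; BP_PlayerController also supplies the hiding state that blocks movement and flashlight, plus a bound light-input event.
; A timeline lerps capsule height for crouching, and Tick scales camera shake by velocity.
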(event Custom|My_Uncrouch
  ;[1 1 1] S'accroupir
  (bind (_direction _time) (Timeline|Crouching Reverse)
    (:Update
      (Components|Capsule|SetCapsuleHalfHeight (Variables|Collision|GetCapsuleComponent) (Math|Float|Lerp (Variables|Size|GetMax%20Size%20Y) (Variables|Size|GetMin%20Size%20Y) _time) true))
    (:Finished
      (if (Utilities|Enum|Equal(Enum) _direction "Backward")
        (Character|UnCrouch)))))

(event Custom|FlashLightEvent
  ;[1 1 1] Flashlight
  (if (not (Variables|/Game/Blueprint/BP_Player/BP_PlayerController.BP_PlayerController_C|GetIsHiding (.AsBP%20Player%20Controller (Utilities|Casting|CastToBP_PlayerController (Game|GetPlayerController 0)))))
    (Utilities|FlowControl|FlipFlop
      (:A
        (Rendering|SetVisibility (Variables|Default|GetTorche) false false))
      (:B
        (Rendering|SetVisibility (Variables|Default|GetTorche) true false)))))

(event Custom|SpeedModifie
  ;[1 1 1] Speed modification
  (if (Variables|Default|GetRun?)
    (Variables|/Script/Engine.CharacterMovementComponent|SetMaxWalkSpeed (Variables|Character|GetCharacterMovement) (select (Variables|/Game/Blueprint/BP_Player/BP_PlayerController.BP_PlayerController_C|GetisMedocTaken (Variables|Components|GetAs%20BP%20Player%20Controller)) (Variables|Speed|GetMax%20Sprint-Crouch%20Speed) (Variables|Speed|GetMax%20Sprint-Walk%20Speed)))
    (Variables|/Script/Engine.CharacterMovementComponent|SetMaxWalkSpeedCrouched (Variables|Character|GetCharacterMovement) (select (Variables|/Game/Blueprint/BP_Player/BP_PlayerController.BP_PlayerController_C|GetisMedocTaken (Variables|Components|GetAs%20BP%20Player%20Controller)) (Variables|Speed|GetMax%20Crouch%20Speed) (Variables|Speed|GetMax%20Sprint-Crouch%20Speed)))
    (if (Variables|Default|GetRun?) :!label _label
      (Default|ModifyHP (Variables|Components|GetAs%20BP%20Player%20Controller) -0.5)
      (Utilities|FlowControl|Delay 0.2)
      (goto _label))
    (else
      (Variables|/Script/Engine.CharacterMovementComponent|SetMaxWalkSpeed (Variables|Character|GetCharacterMovement) (select (Variables|/Game/Blueprint/BP_Player/BP_PlayerController.BP_PlayerController_C|GetisMedocTaken (Variables|Components|GetAs%20BP%20Player%20Controller)) (Variables|Speed|GetMax%20Crouch%20Speed) (Variables|Speed|GetMax%20Walk%20Speed)))
      (Variables|/Script/Engine.CharacterMovementComponent|SetMaxWalkSpeedCrouched (Variables|Character|GetCharacterMovement) (select (Variables|/Game/Blueprint/BP_Player/BP_PlayerController.BP_PlayerController_C|GetisMedocTaken (Variables|Components|GetAs%20BP%20Player%20Controller)) (Variables|Speed|GetMax%20Sprint-Crouch%20Speed) (Variables|Speed|GetMax%20Crouch%20Speed)))
      (if (not (Variables|Default|GetRun?)) :!label _label_2
        (Default|ModifyHP (Variables|Components|GetAs%20BP%20Player%20Controller) 0.2)
        (Utilities|FlowControl|Delay 0.2)
        (goto _label_2)))))

(event EventOnStartCrouch
  (params (HalfHeightAdjust :type Float%20%28single-precision%29) (ScaledHalfHeightAdjust :type Float%20%28single-precision%29))
  ;[1 1 1] S'accroupir
  (bind (_direction _time) (Timeline|Crouching Play)
    (:Update
      (Components|Capsule|SetCapsuleHalfHeight (Variables|Collision|GetCapsuleComponent) (Math|Float|Lerp (Variables|Size|GetMax%20Size%20Y) (Variables|Size|GetMin%20Size%20Y) _time) true))
    (:Finished
      (if (Utilities|Enum|Equal(Enum) _direction "Backward")
        (Character|UnCrouch)))))

(event EventTick
  (params (DeltaSeconds :type Float%20%28single-precision%29))
  (bind _returnvalue (Transformation|GetVelocity))
  (bind _max_sprint_walk_speed (Variables|Speed|GetMax%20Sprint-Walk%20Speed))
  (bind _returnvalue_2 (Math|Vector|VectorLength _returnvalue))
  (bind _returnvalue_3 (Math|Float|Absolute(Float) _returnvalue_2))
  (bind _returnvalue_4 (/ _returnvalue_3 _max_sprint_walk_speed))
  (bind _returnvalue_5 (Math|Float|Lerp 0.0 1.5 _returnvalue_4))
  ;[1 1 1] Camera Shaking / adapter a la vitesse du character
  (Utilities|FlowControl|Delay 0.1)
  (if (> _returnvalue_5 0.01)
    (Game|Feedback|ClientStartCameraShake (Game|GetPlayerController 0) "/Game/Blueprint/BP_Player/BP_cameraShake.BP_cameraShake_C" _returnvalue_5 "CameraLocal" "0, 0, 0")
    (else
      (Game|Feedback|ClientStopCameraShake (Game|GetPlayerController 0) "/Game/Blueprint/BP_Player/BP_cameraShake.BP_cameraShake_C" false))))

(event EventBeginPlay
  (bind _returnvalue (Game|GetPlayerController 0))
  (bind _asbp_player_controller (Utilities|Casting|CastToBP_PlayerController _returnvalue))
  ;[1 1 1] S'accroupir
  ;;[1 1 1] Event begin play
  (bind _asbp_player_controller_2 (Utilities|Casting|CastToBP_PlayerController (Game|GetPlayerController 0)))
  (Variables|Components|SetAs%20BP%20Player%20Controller _asbp_player_controller_2)
  (Components|Timeline|SetPlayRate (Variables|Default|GetCrouching) 1.5)
  (Variables|/Game/Blueprint/BP_Player/BP_PlayerController.BP_PlayerController_C|SetMyPlayer _asbp_player_controller self)
  (EventDispatchers|BindEventtoONLIGHTINPUT _asbp_player_controller (EventDispatchers|CreateEvent :!event Custom|FlashLightEvent)))

(event Input|ActionEvents|InputActionSprint
  (params (Key :type Key%20Structure :default "None"))
  ;[1 1 1] Sprint
  (:Pressed
    (Variables|Default|SetRun? true)
    (CallFunction|SpeedModifie))
  (:Released
    (Variables|Default|SetRun? false)
    (CallFunction|SpeedModifie)))

(event Input|ActionEvents|InputActionInverserlacamera
  (params (Key :type Key%20Structure :default "None"))
  ;[1 1 1] Camera Control
  (:Pressed
    (Utilities|FlowControl|FlipFlop
      (:A
        (Variables|Default|SetInvertion/Cam%20Y -1))
      (:B
        (Variables|Default|SetInvertion/Cam%20Y 1)))))

(event Input|ActionEvents|InputActionCrouch
  (params (Key :type Key%20Structure :default "None"))
  ;[1 1 1] S'accroupir
  (:Pressed
    (Utilities|FlowControl|FlipFlop
      (:A
        (Character|Crouch))
      (:B
        (CallFunction|MyUncrouch)))))

(event Input|AxisEvents|InputAxisLookUp/Down
  (params (AxisValue :type Float%20%28single-precision%29))
  ;[1 1 1] Camera Control
  (Pawn|Input|AddControllerPitchInput (* (Variables|Default|GetInvertion/Cam%20Y) AxisValue)))

(event Input|AxisEvents|InputAxisLookRight/Left
  (params (AxisValue :type Float%20%28single-precision%29))
  ;[1 1 1] Camera Control
  (Pawn|Input|AddControllerYawInput AxisValue))

(event Input|AxisEvents|InputAxisForward/Backward
  (params (AxisValue :type Float%20%28single-precision%29))
  ;[1 1 1] Movement
  (if (not (Variables|/Game/Blueprint/BP_Player/BP_PlayerController.BP_PlayerController_C|GetIsHiding (Variables|Components|GetAs%20BP%20Player%20Controller)))
    (Pawn|Input|AddMovementInput (select (Class|HeadMountedDisplayFunctionLibrary|IsHeadMountedDisplayEnabled) (Math|Vector|GetForwardVector (Variables|Default|GetFirstPersonCamera)) (Transformation|GetActorForwardVector)) AxisValue false)))

(event Input|AxisEvents|InputAxisRight/Left
  (params (AxisValue :type Float%20%28single-precision%29))
  ;[1 1 1] Movement
  (if (not (Variables|/Game/Blueprint/BP_Player/BP_PlayerController.BP_PlayerController_C|GetIsHiding (Variables|Components|GetAs%20BP%20Player%20Controller)))
    (Pawn|Input|AddMovementInput (select (Class|HeadMountedDisplayFunctionLibrary|IsHeadMountedDisplayEnabled) (Math|Vector|GetRightVector (Variables|Default|GetFirstPersonCamera)) (Transformation|GetActorRightVector)) AxisValue false)))

(event Input|KeyboardEvents|Escape
  (params (Key :type Key%20Structure :default "None"))
  (bind _returnvalue (Game|GetPlayerController 0))
  ;[1 1 1] Esc menu
  (:Pressed
    (Utilities|FlowControl|FlipFlop
      (:A
        (bind _returnvalue_2 (UserInterface|CreateWidget "/Game/Blueprint/UI/WBP_EchapMenu.WBP_EchapMenu_C"))
        (UserInterface|Viewport|AddtoViewport _returnvalue_2 0)
        (Game|SetGamePaused true)
        (Variables|/Script/Engine.PlayerController|SetbShowMouseCursor _returnvalue true))
      (:B
        (Widget|RemovefromParent _returnvalue_2)
        (Game|SetGamePaused false)
        (Variables|/Script/Engine.PlayerController|SetbShowMouseCursor _returnvalue false)))))

(fn ConstructionScript)

(fn Dead
  (CallFunction|Dead))