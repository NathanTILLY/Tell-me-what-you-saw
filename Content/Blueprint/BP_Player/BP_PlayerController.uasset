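; Player controller for a horror game that manages sanity as health, shows its bar widget and forwards interact and flashlight input.
; Stats live in a BP_PlayerStats SaveGame object on LifeGameInstance, created on demand; SaveStats is empty.
; Medication counts uses, restores sanity, flashes the screen and shares StunTrap's timed IsHiding state.
; Tick plays a one-time sound when IsHiding is set and sanity is below maximum.
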(event Custom|SaveStats)

(event Custom|CreatePlayerStats
  (bind _aslife_game_instance (Utilities|Casting|CastToLifeGameInstance (Game|GetGameInstance)))
  (Utilities|IsValid (Variables|/Game/Blueprint/GameInstance/LifeGameInstance.LifeGameInstance_C|GetPlayerStats _aslife_game_instance)
    (:Is%20Not%20Valid
      (bind _returnvalue (SaveGame|CreateSaveGameObject "/Game/Blueprint/BP_Player/BP_PlayerStats.BP_PlayerStats_C"))
      (Variables|/Game/Blueprint/GameInstance/LifeGameInstance.LifeGameInstance_C|SetPlayerStats _aslife_game_instance _returnvalue))))

(event Custom|Stun%20Trap
  (Variables|Default|SetIsHiding true)
  (Utilities|FlowControl|Delay 3.0)
  (Variables|Default|SetIsHiding false))

(event EventBeginPlay
  (Utilities|FlowControl|Sequence
    (:then_0
      (CallFunction|BarreVie))
    (:then_1
      (if (Variables|Default|GetIsDecreasing)
        _))
    (:then_2
      (bind _aslife_game_instance (Utilities|Casting|CastToLifeGameInstance (Game|GetGameInstance)))
      (Development|PrintString (Utilities|String|ToString(Boolean) (Utilities|IsValid (Variables|/Game/Blueprint/GameInstance/LifeGameInstance.LifeGameInstance_C|GetPlayerStats _aslife_game_instance)))))
    (:then_3
      (CallFunction|CreatePlayerStats))))

(event EventTick
  (params (DeltaSeconds :type Float%20%28single-precision%29))
  ;[1 1 1] Sound after he see the monster Once
  (Utilities|FlowControl|Delay 0.2)
  (if (!= (Variables|Default|GetSanityActuelle) (Variables|Default|GetSanityMax))
    (if (Variables|Default|GetIsHiding)
      (Utilities|FlowControl|DoOnce false
        (:Completed
          (Development|PrintString "Sound appears")
          (Audio|PlaySound2D 0 1.0 1.0 0.0 0 0))))))

(event Input|ActionEvents|InputActionMedicament
  (params (Key :type Key%20Structure :default "None"))
  (:Pressed
    (Math|Integer|IncrementInt (Variables|/Game/Blueprint/BP_Player/BP_PlayerStats.BP_PlayerStats_C|GetMedocPris (CallFunction|GetStats))
      (:%20%20
        (CallFunction|ModifyHP 3e+01)
        (Utilities|FlowControl|Sequence
          (:then_0
            (Variables|Default|SetIsHiding true)
            (Utilities|FlowControl|Delay 3.0)
            (Variables|Default|SetIsHiding false))
          (:then_1
            (bind _returnvalue (UserInterface|CreateWidget "/Game/Blueprint/UI/WBP_Flash.WBP_Flash_C"))
            (UserInterface|Viewport|AddtoViewport _returnvalue 0)))))))

(event Input|ActionEvents|InputActionInteract
  (params (Key :type Key%20Structure :default "None"))
  (:Pressed
    (Default|CallONINTERACT)))

(event Input|ActionEvents|InputActionFlashLight
  (params (Key :type Key%20Structure :default "None"))
  (:Pressed
    (Default|CallONLIGHTINPUT)))

(fn ConstructionScript)

(fn OuvrirPorte)

(fn BarreVie
  (bind _returnvalue (UserInterface|CreateWidget "/Game/Blueprint/UI/WBP_Vie.WBP_Vie_C" 0 self))
  (bind _output_get (Variables|Default|SetHealthBarReference _returnvalue))
  (UserInterface|Viewport|AddtoViewport _output_get 0))

(fn ModifyHP
  (params (amount :type Float%20%28single-precision%29))
  (bind _playerstats (CallFunction|GetStats))
  (Variables|/Game/Blueprint/BP_Player/BP_PlayerStats.BP_PlayerStats_C|SetSanityActuelle _playerstats (Math|Float|Clamp(Float) (+ amount (Variables|/Game/Blueprint/BP_Player/BP_PlayerStats.BP_PlayerStats_C|GetSanityActuelle _playerstats)) 0.0 (Variables|Default|GetSanityMax)))
  (bind _healthbarreference (Variables|Default|GetHealthBarReference)
    (:then
      (Default|UpdatePercentage _healthbarreference))
    (:else)))

(fn ModifyHP2
  (params (Amount :type Float%20%28single-precision%29))
  (Variables|/Game/Blueprint/GameInstance/LifeGameInstance.LifeGameInstance_C|SetSanityActuelle (.AsLife%20Game%20Instance (Utilities|Casting|CastToLifeGameInstance (Game|GetGameInstance))) (Math|Float|Clamp(Float) (+ Amount (Variables|/Game/Blueprint/GameInstance/LifeGameInstance.LifeGameInstance_C|GetSanityActuelle (.AsLife%20Game%20Instance (Utilities|Casting|CastToLifeGameInstance (Game|GetGameInstance))))) 0.0 (Variables|Default|GetSanityMax)))
  (bind _healthbarreference (Variables|Default|GetHealthBarReference)
    (:then
      (Default|UpdatePercentage _healthbarreference))
    (:else)))

(fn GetStats
  (bind _playerstats (Variables|/Game/Blueprint/GameInstance/LifeGameInstance.LifeGameInstance_C|GetPlayerStats (.AsLife%20Game%20Instance (Utilities|Casting|CastToLifeGameInstance (Game|GetGameInstance))))
    (:then
      _)
    (:else
      (CallFunction|CreatePlayerStats)))
  (return _playerstats))