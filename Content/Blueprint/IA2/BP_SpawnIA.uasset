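; BP_SpawnIA is a spawner actor that keeps the level populated with BP_Creature AI.
; On Tick it counts all creatures in the world and, when fewer than two exist, waits through a one-second Delay.
; It then spawns a BP_Creature running BT_Creature at a random point inside its Box component's bounds.
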(event EventTick
  (params (DeltaSeconds :type Float%20%28single-precision%29))
  (bind _box (Variables|Default|GetBox))
  (if true
    (bind _outactors (Actor|GetAllActorsOfClass "/Game/Blueprint/IA2/BP_Creature.BP_Creature_C"))
    (if (< (Utilities|Array|Length _outactors) 2)
      (Utilities|FlowControl|Delay 1.0)
      (AI|SpawnAIFromClass "/Game/Blueprint/IA2/BP_Creature.BP_Creature_C" "/Game/Blueprint/IA2/BT_Creature.BT_Creature" (Math|Random|RandomPointinBoundingBox (Transformation|GetWorldLocation _box) (Components|Box|GetScaledBoxExtent _box)) "0, 0, 0" false 0))))

(fn ConstructionScript)