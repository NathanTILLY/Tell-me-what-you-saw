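; Trigger volume that spawns a Jumeaux (twins) creature when the player pawn enters it while the player controller's HasKeyOLD flag is set.
; Each qualifying overlap counts the existing BP_Creature_Jumeaux actors in the level and spawns one more only while that count is below NumberToSpawn.
; The creature spawns with the BT_Creature behavior tree at the location and rotation of the SpawnerLocation1 actor.
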(event OnComponentBeginOverlap(Box)
  (params (OverlappedComponent :type Primitive%20Component%20Object%20Reference) (OtherActor :type Actor%20Object%20Reference) (OtherComp :type Primitive%20Component%20Object%20Reference) (OtherBodyIndex :type Integer) (bFromSweep :type Boolean) (SweepResult :type Hit%20Result%20Structure%20%28by%20ref%29))
  (bind _spawnerlocation1 (Variables|Default|GetSpawnerLocation1))
  (bind _rootcomponent (Variables|/Script/Engine.Actor|GetRootComponent _spawnerlocation1))
  (if (== OtherActor (Game|Player|GetPlayerPawn 0))
    (if (Variables|/Game/Blueprint/BP_Player/BP_PlayerController.BP_PlayerController_C|GetHasKeyOLD (.AsBP%20Player%20Controller (Utilities|Casting|CastToBP_PlayerController (Game|GetPlayerController 0))))
      (bind _outactors (Actor|GetAllActorsOfClass "/Game/Blueprint/IA2/BP_Creature_Jumeaux.BP_Creature_Jumeaux_C"))
      (if (< (Utilities|Array|Length _outactors) (Variables|Default|GetNumber%20to%20Spawn))
        (AI|SpawnAIFromClass "/Game/Blueprint/IA2/BP_Creature_Jumeaux.BP_Creature_Jumeaux_C" "/Game/Blueprint/IA2/BT_Creature.BT_Creature" (Transformation|GetWorldLocation _rootcomponent) (Transformation|GetWorldRotation _rootcomponent) false 0)))))

(fn ConstructionScript)