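; BP_Monstre_2_Malicieux is a monster Blueprint with a touch-to-kill trigger for the player.
; When BP_Player begins overlapping TouchThatYourDead, it reads IsHiding on BP_PlayerController and only prints "Dead" if the player is not hiding.
; A disconnected chain that would show the death and end-of-game widgets, pause the game and show the cursor never runs.
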(event OnComponentBeginOverlap(TouchThatYourDead)
  (params (OverlappedComponent :type Primitive%20Component%20Object%20Reference) (OtherActor :type Actor%20Object%20Reference) (OtherComp :type Primitive%20Component%20Object%20Reference) (OtherBodyIndex :type Integer) (bFromSweep :type Boolean) (SweepResult :type Hit%20Result%20Structure%20%28by%20ref%29))
  (Utilities|Casting|CastToBP_Player OtherActor)
  (if (not (Variables|/Game/Blueprint/BP_Player/BP_PlayerController.BP_PlayerController_C|GetIsHiding (.AsBP%20Player%20Controller (Utilities|Casting|CastToBP_PlayerController (Game|GetPlayerController 0)))))
    (Development|PrintString "Dead")))

(fn ConstructionScript)