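; BP_SpawnIA_Jumeaux is a trigger that spawns BP_Creature_Jumeaux AI running BT_Creature when the player pawn overlaps its Box.
; Each overlap spawns up to two creatures, at the transforms of SpawnerLocation1 and then SpawnerLocation2.
; Before each spawn, it counts every such creature in the world against NumberToSpawn, so the cap is global and the trigger can refill on later overlaps.
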(event OnComponentBeginOverlap(Box)
  (params (OverlappedComponent :type Primitive%20Component%20Object%20Reference) (OtherActor :type Actor%20Object%20Reference) (OtherComp :type Primitive%20Component%20Object%20Reference) (OtherBodyIndex :type Integer) (bFromSweep :type Boolean) (SweepResult :type Hit%20Result%20Structure%20%28by%20ref%29))
  (bind _spawnerlocation1 (Variables|Default|GetSpawnerLocation1))
  (bind _spawnerlocation2 (Variables|Default|GetSpawnerLocation2))
  (bind _rootcomponent (Variables|/Script/Engine.Actor|GetRootComponent _spawnerlocation2))
  (bind _rootcomponent_2 (Variables|/Script/Engine.Actor|GetRootComponent _spawnerlocation1))
  (if (== OtherActor (Game|Player|GetPlayerPawn 0))
    (bind _outactors (Actor|GetAllActorsOfClass "/Game/Blueprint/IA2/BP_Creature_Jumeaux.BP_Creature_Jumeaux_C"))
    (if (< (Utilities|Array|Length _outactors) (Variables|Default|GetNumber%20to%20Spawn))
      (AI|SpawnAIFromClass "/Game/Blueprint/IA2/BP_Creature_Jumeaux.BP_Creature_Jumeaux_C" "/Game/Blueprint/IA2/BT_Creature.BT_Creature" (Transformation|GetWorldLocation _rootcomponent_2) (Transformation|GetWorldRotation _rootcomponent_2) false 0)
      (bind _outactors_2 (Actor|GetAllActorsOfClass "/Game/Blueprint/IA2/BP_Creature_Jumeaux.BP_Creature_Jumeaux_C"))
      (if (< (Utilities|Array|Length _outactors_2) (Variables|Default|GetNumber%20to%20Spawn))
        (AI|SpawnAIFromClass "/Game/Blueprint/IA2/BP_Creature_Jumeaux.BP_Creature_Jumeaux_C" "/Game/Blueprint/IA2/BT_Creature.BT_Creature" (Transformation|GetWorldLocation _rootcomponent) (Transformation|GetWorldRotation _rootcomponent) false 0)))))

(fn ConstructionScript)