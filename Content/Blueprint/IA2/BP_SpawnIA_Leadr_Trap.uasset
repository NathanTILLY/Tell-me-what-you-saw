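; Trap volume that springs a Leadr creature on the player, stunning them when they enter the box.
; On the first player overlap, if fewer Leadr creatures than NumberToSpawn exist, it spawns one at SpawnerLocation1 running BT_Creature.
; It then calls StunTrap on the player controller and plays a collapse sound.
; After a delay, it destroys every Leadr creature in the level, including any it did not spawn.
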(event OnComponentBeginOverlap(Box)
  (params (OverlappedComponent :type Primitive%20Component%20Object%20Reference) (OtherActor :type Actor%20Object%20Reference) (OtherComp :type Primitive%20Component%20Object%20Reference) (OtherBodyIndex :type Integer) (bFromSweep :type Boolean) (SweepResult :type Hit%20Result%20Structure%20%28by%20ref%29))
  (bind _spawnerlocation1 (Variables|Default|GetSpawnerLocation1))
  (bind _rootcomponent (Variables|/Script/Engine.Actor|GetRootComponent _spawnerlocation1))
  (if (== OtherActor (Game|Player|GetPlayerPawn 0))
    (Utilities|FlowControl|DoOnce false
      (:Completed
        (bind _outactors (Actor|GetAllActorsOfClass "/Game/Blueprint/IA2/BP_Creature_Leadr.BP_Creature_Leadr_C"))
        (if (< (Utilities|Array|Length _outactors) (Variables|Default|GetNumber%20to%20Spawn))
          (AI|SpawnAIFromClass "/Game/Blueprint/IA2/BP_Creature_Leadr.BP_Creature_Leadr_C" "/Game/Blueprint/IA2/BT_Creature.BT_Creature" (Transformation|GetWorldLocation _rootcomponent) (Transformation|GetWorldRotation _rootcomponent) false 0)
          (bind _asbp_player_controller (Utilities|Casting|CastToBP_PlayerController (Game|GetPlayerController 0)))
          (Default|StunTrap _asbp_player_controller)
          (Audio|PlaySound2D "/Game/StarterContent/Audio/Collapse01.Collapse01" 1.0 1.0 0.0 0 0)
          (Utilities|FlowControl|Delay 1e+01)
          (bind _outactors_2 (Actor|GetAllActorsOfClass "/Game/Blueprint/IA2/BP_Creature_Leadr.BP_Creature_Leadr_C"))
          (Actor|DestroyActor _outactors_2))))))

(fn ConstructionScript)