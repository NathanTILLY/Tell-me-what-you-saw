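; AI controller for a creature that runs the BT_Creature behavior tree when play begins.
; On each perception update it writes the perceived actor to the TargetActor blackboard key, without checking whether the actor was sensed or lost.
; If the first player controller's IsHiding flag is set at that moment, it clears the key instead.
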(event OnTargetPerceptionUpdated(AIPerception)
  (params (Actor :type Actor%20Object%20Reference) (Stimulus :type AI%20Stimulus%20Structure))
  (if (Variables|/Game/Blueprint/BP_Player/BP_PlayerController.BP_PlayerController_C|GetIsHiding (.AsBP%20Player%20Controller (Utilities|Casting|CastToBP_PlayerController (Game|GetPlayerController 0))))
    (AI|Components|Blackboard|SetValueasObject (Variables|Default|GetBlackboard) (Utilities|Name|MakeLiteralName "TargetActor") 0)
    (else
      (AI|Components|Blackboard|SetValueasObject (Variables|Default|GetBlackboard) (Utilities|Name|MakeLiteralName "TargetActor") Actor))))

(event EventBeginPlay
  (AI|RunBehaviorTree "/Game/Blueprint/IA2/BT_Creature.BT_Creature"))

(fn ConstructionScript)