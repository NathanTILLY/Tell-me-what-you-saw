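; Static Jumeaux (twins) creature that drains the player's sanity nearby and kills on touch.
; Overlapping TouchThatYourDead while the player is not hiding shows the death and game-over widgets, pauses the game and shows the cursor.
; Sphere overlaps toggle the controller's IsDecreasing flag for any actor, before the player cast.
; For the player, that flag gates Delay-based loops calling ModifyHP, draining quickly inside and recovering slowly after exit.
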(event OnComponentBeginOverlap(TouchThatYourDead)
  (params (OverlappedComponent :type Primitive%20Component%20Object%20Reference) (OtherActor :type Actor%20Object%20Reference) (OtherComp :type Primitive%20Component%20Object%20Reference) (OtherBodyIndex :type Integer) (bFromSweep :type Boolean) (SweepResult :type Hit%20Result%20Structure%20%28by%20ref%29))
  (Utilities|Casting|CastToBP_Player OtherActor)
  (if (not (Variables|/Game/Blueprint/BP_Player/BP_PlayerController.BP_PlayerController_C|GetIsHiding (.AsBP%20Player%20Controller (Utilities|Casting|CastToBP_PlayerController (Game|GetPlayerController 0)))))
    (bind _returnvalue (UserInterface|CreateWidget "/Game/Blueprint/UI/WBP_Death.WBP_Death_C"))
    (UserInterface|Viewport|AddtoViewport _returnvalue 0)
    (bind _returnvalue_2 (UserInterface|CreateWidget "/Game/Blueprint/UI/WBP_FinDePartie.WBP_FinDePartie_C"))
    (UserInterface|Viewport|AddtoViewport _returnvalue_2 0)
    (Game|SetGamePaused true)
    (Variables|/Script/Engine.PlayerController|SetbShowMouseCursor (Game|GetPlayerController 0) true)))

(event OnComponentBeginOverlap(Sphere)
  (params (OverlappedComponent :type Primitive%20Component%20Object%20Reference) (OtherActor :type Actor%20Object%20Reference) (OtherComp :type Primitive%20Component%20Object%20Reference) (OtherBodyIndex :type Integer) (bFromSweep :type Boolean) (SweepResult :type Hit%20Result%20Structure%20%28by%20ref%29))
  (bind _returnvalue (Game|GetPlayerController 0))
  (bind _asbp_player_controller (Utilities|Casting|CastToBP_PlayerController _returnvalue))
  ;[1 1 1] sanity decrease
  (Utilities|FlowControl|Sequence
    (:then_0
      (Variables|/Game/Blueprint/BP_Player/BP_PlayerController.BP_PlayerController_C|SetIsDecreasing (.AsBP%20Player%20Controller (Utilities|Casting|CastToBP_PlayerController (Game|GetPlayerController 0))) true))
    (:then_1
      (Utilities|Casting|CastToBP_Player OtherActor)
      (if (Variables|/Game/Blueprint/BP_Player/BP_PlayerController.BP_PlayerController_C|GetIsDecreasing _asbp_player_controller) :!label _label
        (Default|ModifyHP _asbp_player_controller -0.5)
        (Utilities|FlowControl|Delay 0.2)
        (goto _label)))))

(event OnComponentEndOverlap(Sphere)
  (params (OverlappedComponent :type Primitive%20Component%20Object%20Reference) (OtherActor :type Actor%20Object%20Reference) (OtherComp :type Primitive%20Component%20Object%20Reference) (OtherBodyIndex :type Integer))
  (bind _returnvalue (Game|GetPlayerController 0))
  (bind _asbp_player_controller (Utilities|Casting|CastToBP_PlayerController _returnvalue))
  ;[1 1 1] Sanity increase
  (Utilities|FlowControl|Sequence
    (:then_0
      (Variables|/Game/Blueprint/BP_Player/BP_PlayerController.BP_PlayerController_C|SetIsDecreasing (.AsBP%20Player%20Controller (Utilities|Casting|CastToBP_PlayerController (Game|GetPlayerController 0))) false))
    (:then_1
      (Utilities|Casting|CastToBP_Player OtherActor)
      (if (not (Variables|/Game/Blueprint/BP_Player/BP_PlayerController.BP_PlayerController_C|GetIsDecreasing _asbp_player_controller)) :!label _label
        (Default|ModifyHP _asbp_player_controller 0.05)
        (Utilities|FlowControl|Delay 0.2)
        (goto _label)))))

(fn ConstructionScript)