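; BP_FinJeu is an end-of-game trigger that plays the final cinematic and then quits the game.
; BeginPlay creates a Level Sequence player for CinematicFin.
; When the player pawn overlaps the Box, its input is disabled, the pawn is destroyed, and the sequence plays.
; A timer set to the sequence's duration then fires OnEnd, which calls QuitGame.
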(event OnComponentBeginOverlap(Box)
  (params (OverlappedComponent :type Primitive%20Component%20Object%20Reference) (OtherActor :type Actor%20Object%20Reference) (OtherComp :type Primitive%20Component%20Object%20Reference) (OtherBodyIndex :type Integer) (bFromSweep :type Boolean) (SweepResult :type Hit%20Result%20Structure%20%28by%20ref%29))
  (bind _returnvalue (Game|Player|GetPlayerPawn 0))
  (bind _cinematicend (Variables|Default|GetCinematicEnd))
  (if (== OtherActor _returnvalue)
    (Input|DisableInput _returnvalue (Game|GetPlayerController 0))
    (Actor|DestroyActor _returnvalue)
    (Sequencer|Player|Play _cinematicend :!class /Script/MovieScene.MovieSceneSequencePlayer)
    (Utilities|Time|SetTimerbyEvent (delegate Custom|On%20End) (Class|TimeManagementBlueprintLibrary|ToSeconds(QualifiedFrameTime) (Media|MediaPlayer|GetDuration _cinematicend)))))

(event Custom|On%20End
  (Game|QuitGame 0 "Quit" false))

(event EventBeginPlay
  (bind _returnvalue (Sequencer|Player|CreateLevelSequencePlayer "/Game/Animations/Cinematics/CinematicFin.CinematicFin"))
  (Variables|Default|SetCinematicEnd _returnvalue))

(fn ConstructionScript)