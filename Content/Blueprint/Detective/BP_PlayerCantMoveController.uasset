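; BP_PlayerCantMoveController is a Detective player controller, named for a player who cannot move, that manages health and its on-screen bar.
; BarreVie creates the WBP_Vie widget, stores it and adds it to the viewport.
; ModifyHP clamps VieActuelle between zero and VieMax, then refreshes the bar's percentage.
; OuvrirPorte is an empty stub, and the FlashLightEvent call in the event graph never runs.
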(fn ConstructionScript)

(fn OuvrirPorte)

(fn BarreVie
  (bind _returnvalue (UserInterface|CreateWidget "/Game/Blueprint/UI/WBP_Vie.WBP_Vie_C" 0 self))
  (bind _output_get (Variables|Default|SetHealthBarReference _returnvalue))
  (UserInterface|Viewport|AddtoViewport _output_get 0))

(fn ModifyHP
  (params (amount :type Integer))
  (Variables|Default|SetVieActuelle (Math|Integer|Clamp(Integer) (+ amount (Variables|Default|GetVieActuelle)) 0 (Variables|Default|GetVieMax)))
  (Default|UpdatePercentage (Variables|Default|GetHealthBarReference)))