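; Inspector character for the detective game that plays a scripted animation sequence suited to the current level.
; On BeginPlay it checks the level name and sets a starting pose on Inspector_AnimBP.
; Level1 and Level2 then step through chains of Delays that toggle AnimBP flags for gestures, reading and dialog, while any other level only gets a pose.
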(event EventBeginPlay
  (bind _returnvalue (Game|GetCurrentLevelName true))
  (Variables|Default|SetLevel _returnvalue)
  (if (Utilities|Enum|Equal(Enum) (Variables|Default|GetLevel) (Variables|Default|GetLevel1))
    (Variables|/Game/Animations/Inspector_AnimBP.Inspector_AnimBP_C|Setpose (CallFunction|GetAnimBP) "NewEnumerator0")
    (Utilities|FlowControl|Delay 2.0)
    (bind _asinspector_anim_bp (Utilities|Casting|CastToInspector_AnimBP (Components|SkeletalMesh|GetAnimInstance (Variables|Default|GetSkeletalMesh))))
    (Variables|/Game/Animations/Inspector_AnimBP.Inspector_AnimBP_C|SetRiseArms _asinspector_anim_bp true)
    (Utilities|FlowControl|Delay 2.0)
    (bind _asinspector_anim_bp_2 (Utilities|Casting|CastToInspector_AnimBP (Components|SkeletalMesh|GetAnimInstance (Variables|Default|GetSkeletalMesh))))
    (Variables|/Game/Animations/Inspector_AnimBP.Inspector_AnimBP_C|SetLowerArms _asinspector_anim_bp_2 true)
    (Utilities|FlowControl|Delay 5.0)
    (bind _asinspector_anim_bp_3 (Utilities|Casting|CastToInspector_AnimBP (Components|SkeletalMesh|GetAnimInstance (Variables|Default|GetSkeletalMesh))))
    (Variables|/Game/Animations/Inspector_AnimBP.Inspector_AnimBP_C|SetCanRead _asinspector_anim_bp_3 true)
    (Utilities|FlowControl|Delay 2.0)
    (bind _asinspector_anim_bp_4 (Utilities|Casting|CastToInspector_AnimBP (Components|SkeletalMesh|GetAnimInstance (Variables|Default|GetSkeletalMesh))))
    (Variables|/Game/Animations/Inspector_AnimBP.Inspector_AnimBP_C|SetCanDialog _asinspector_anim_bp_4 true)
    (elif (Utilities|Enum|Equal(Enum) (Variables|Default|GetLevel) (Variables|Default|GetLevel2))
      (Variables|/Game/Animations/Inspector_AnimBP.Inspector_AnimBP_C|Setpose (CallFunction|GetAnimBP) "NewEnumerator1")
      (Utilities|FlowControl|Delay 2.0)
      (bind _asinspector_anim_bp_5 (Utilities|Casting|CastToInspector_AnimBP (Components|SkeletalMesh|GetAnimInstance (Variables|Default|GetSkeletalMesh))))
      (Variables|/Game/Animations/Inspector_AnimBP.Inspector_AnimBP_C|SetRires _asinspector_anim_bp_5 true)
      (Utilities|FlowControl|Delay 2.0)
      (bind _asinspector_anim_bp_6 (Utilities|Casting|CastToInspector_AnimBP (Components|SkeletalMesh|GetAnimInstance (Variables|Default|GetSkeletalMesh))))
      (Variables|/Game/Animations/Inspector_AnimBP.Inspector_AnimBP_C|SetCanDialog2 _asinspector_anim_bp_6 true)
      (Utilities|FlowControl|Delay 2.0)
      (bind _asinspector_anim_bp_7 (Utilities|Casting|CastToInspector_AnimBP (Components|SkeletalMesh|GetAnimInstance (Variables|Default|GetSkeletalMesh))))
      (Variables|/Game/Animations/Inspector_AnimBP.Inspector_AnimBP_C|SetCanDialog3 _asinspector_anim_bp_7 false)
      (else
        (Variables|/Game/Animations/Inspector_AnimBP.Inspector_AnimBP_C|Setpose (CallFunction|GetAnimBP) "NewEnumerator2")))))

(fn ConstructionScript)

(fn GetAnimBP
  (return (.AsInspector%20Anim%20BP (Utilities|Casting|CastToInspector_AnimBP (Components|SkeletalMesh|GetAnimInstance (Variables|Default|GetSkeletalMesh))))))