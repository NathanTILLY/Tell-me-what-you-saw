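; BP_PlayerCantMove is a player Blueprint in the Detective folder that handles looking around and the pause menu, with no movement input of its own.
; Look axes drive controller pitch and yaw, with yaw then clamped between MinYaw and MaxYaw through SetControlRotation.
; An input action toggles vertical camera inversion via a FlipFlop.
; Escape flip-flops WBP_EchapMenu, game pause and mouse cursor together.
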(event Input|ActionEvents|InputActionInverserlacamera
  (params (Key :type Key%20Structure :default "None"))
  ;[1 1 1] Camera Control
  (:Pressed
    (Utilities|FlowControl|FlipFlop
      (:A
        (Variables|Default|SetInvertion/Cam%20Y -1))
      (:B
        (Variables|Default|SetInvertion/Cam%20Y 1)))))

(event Input|AxisEvents|InputAxisLookUp/Down
  (params (AxisValue :type Float%20%28single-precision%29))
  ;[1 1 1] Camera Control
  (Pawn|Input|AddControllerPitchInput (* (Variables|Default|GetInvertion/Cam%20Y) AxisValue)))

(event Input|AxisEvents|InputAxisLookRight/Left
  (params (AxisValue :type Float%20%28single-precision%29))
  (bind _returnvalue (Pawn|GetControlRotation :!class /Script/Engine.Pawn))
  ;[1 1 1] Camera Control
  (Pawn|Input|AddControllerYawInput AxisValue)
  (Pawn|SetControlRotation (Game|GetPlayerController 0) (Math|Rotator|MakeRotator (.roll _returnvalue) (.pitch _returnvalue) (Class|KismetMathLibrary|ClampAxis (Math|Float|ClampAngle (+ AxisValue (.yaw _returnvalue)) (Variables|Default|GetMinYaw) (Variables|Default|GetMaxYaw))))))

(event Input|KeyboardEvents|Escape
  (params (Key :type Key%20Structure :default "None"))
  (bind _returnvalue (Game|GetPlayerController 0))
  ;[1 1 1] Esc menu
  (:Pressed
    (Utilities|FlowControl|FlipFlop
      (:A
        (bind _returnvalue_2 (UserInterface|CreateWidget "/Game/Blueprint/UI/WBP_EchapMenu.WBP_EchapMenu_C"))
        (UserInterface|Viewport|AddtoViewport _returnvalue_2 0)
        (Game|SetGamePaused true)
        (Variables|/Script/Engine.PlayerController|SetbShowMouseCursor _returnvalue true))
      (:B
        (Widget|RemovefromParent _returnvalue_2)
        (Game|SetGamePaused false)
        (Variables|/Script/Engine.PlayerController|SetbShowMouseCursor _returnvalue false)))))

(fn ConstructionScript)

(fn Dead
  (CallFunction|Dead))