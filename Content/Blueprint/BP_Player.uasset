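; BP_Player is the first-person player character Blueprint, handling look, movement, crouch and a flashlight.
; Axis inputs drive controller pitch and yaw, plus movement along actor forward and right vectors, or the FirstPersonCamera's vectors when a head-mounted display is enabled.
; FlipFlops turn the crouch and flashlight inputs into toggles, the latter switching visibility of the Torche component.
; The Sprint section is empty.
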(event EventOnStartCrouch
  (params (HalfHeightAdjust :type Float%20%28single-precision%29) (ScaledHalfHeightAdjust :type Float%20%28single-precision%29)))

(event Input|ActionEvents|InputActionFlashLight
  (params (Key :type Key%20Structure :default "None"))
  ;[1 1 1] Flashlight
  (:Pressed
    (Utilities|FlowControl|FlipFlop
      (:A
        (Rendering|SetVisibility (Variables|Default|GetTorche) true false))
      (:B
        (Rendering|SetVisibility (Variables|Default|GetTorche) false false)))))

(event Input|ActionEvents|InputActionCrouch
  (params (Key :type Key%20Structure :default "None"))
  ;[1 1 1] S'accroupir
  (:Pressed
    (Utilities|FlowControl|FlipFlop
      (:A
        (Character|Crouch))
      (:B
        (Character|UnCrouch)))))

(event Input|ActionEvents|InputActionSprint
  (params (Key :type Key%20Structure :default "None"))
  ;[1 1 1] Sprint
)

(event Input|AxisEvents|InputAxisLookUp/Down
  (params (AxisValue :type Float%20%28single-precision%29))
  ;[1 1 1] Camera Control
  (Pawn|Input|AddControllerPitchInput self AxisValue))

(event Input|AxisEvents|InputAxisLookRight/Left
  (params (AxisValue :type Float%20%28single-precision%29))
  ;[1 1 1] Camera Control
  (Pawn|Input|AddControllerYawInput self AxisValue))

(event Input|AxisEvents|InputAxisForward/Backward
  (params (AxisValue :type Float%20%28single-precision%29))
  ;[1 1 1] Movement
  (Pawn|Input|AddMovementInput (select (Class|HeadMountedDisplayFunctionLibrary|IsHeadMountedDisplayEnabled) (Math|Vector|GetForwardVector (Variables|Default|GetFirstPersonCamera)) (Transformation|GetActorForwardVector)) AxisValue false))

(event Input|AxisEvents|InputAxisRight/Left
  (params (AxisValue :type Float%20%28single-precision%29))
  ;[1 1 1] Movement
  (Pawn|Input|AddMovementInput (select (Class|HeadMountedDisplayFunctionLibrary|IsHeadMountedDisplayEnabled) (Math|Vector|GetRightVector (Variables|Default|GetFirstPersonCamera)) (Transformation|GetActorRightVector)) AxisValue false))

(fn ConstructionScript)