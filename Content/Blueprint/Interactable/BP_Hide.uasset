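; BP_Hide is an interactable hiding spot with a door that lets the player hide and come back out.
; Interact calls ToggleHide, which flips IsHiding, visibility and collision on the referenced player object and blends the camera view between the hiding spot and the player.
; Each interaction also plays a timeline from the start that rotates the door's yaw between its closed and open angles.
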(event EventInteract
  (Utilities|FlowControl|Sequence
    (:then_0
      (CallFunction|ToggleHide))
    (:then_1
      ;[1 1 1] Open/close door animation
      (bind _doortrack (Timeline|OpenCloseDoor PlayFromStart)
        (:Update
          (Transformation|SetRelativeRotation (Variables|Default|GetPorte) (Math|Rotator|MakeRotator 0.0 0.0 (Math|Float|Lerp (Variables|Default|GetClosedAngle) (Variables|Default|GetOpenAngle) _doortrack)) false false))))))

(fn ConstructionScript
  (|CallParentFunction))

(fn ToggleHide
  (bind _returnvalue (Game|GetPlayerController 0))
  (bind _as_bp_player_controller (Variables|Default|GetAs%20BP%20Player%20Controller))
  (if (Variables|/Game/Blueprint/BP_Player/BP_PlayerController.BP_PlayerController_C|GetIsHiding (Variables|Default|GetAs%20BP%20Player%20Controller))
    (Variables|/Game/Blueprint/BP_Player/BP_PlayerController.BP_PlayerController_C|SetIsHiding (Variables|Default|GetAs%20BP%20Player%20Controller) false)
    (Rendering|SetActorHiddenInGame _as_bp_player_controller false)
    (Collision|SetActorEnableCollision _as_bp_player_controller true)
    (Game|Player|SetViewTargetwithBlend _returnvalue (Variables|Default|GetAsBP_Player) 0.6 "VTBlend_Linear" 0.0 false)
    (else
      (Variables|/Game/Blueprint/BP_Player/BP_PlayerController.BP_PlayerController_C|SetIsHiding (Variables|Default|GetAs%20BP%20Player%20Controller) true)
      (Rendering|SetActorHiddenInGame _as_bp_player_controller true)
      (Collision|SetActorEnableCollision _as_bp_player_controller false)
      (Game|Player|SetViewTargetwithBlend _returnvalue self 0.6 "VTBlend_Linear" 0.0 false))))