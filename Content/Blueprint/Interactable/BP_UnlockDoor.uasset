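; Interactable unlocked door that swings open and closed, and can also be opened by the BP_Creature_Gros creature.
; Interact flip-flops between playing and reversing a timeline that lerps the door's yaw between closed and open angles.
; A box overlap by the creature, ignoring components tagged SphereIA, plays the timeline if IsDoorOpen is false.
; That flag is set on opening but never cleared here.
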(event OnComponentBeginOverlap(Box)
  (params (OverlappedComponent :type Primitive%20Component%20Object%20Reference) (OtherActor :type Actor%20Object%20Reference) (OtherComp :type Primitive%20Component%20Object%20Reference) (OtherBodyIndex :type Integer) (bFromSweep :type Boolean) (SweepResult :type Hit%20Result%20Structure%20%28by%20ref%29))
  (Utilities|Casting|CastToBP_Creature_Gros OtherActor)
  (if (not (Utilities|Array|ContainsItem (Variables|/Script/Engine.ActorComponent|GetComponentTags OtherComp) "SphereIA"))
    (if (not (Variables|Default|GetIsDoorOpen))
      ;[1 1 1] Open/close door animation
      (bind _doortrack (Timeline|Timeline_0 Play)
        (:Update
          (Transformation|SetRelativeRotation (Variables|Default|GetPorte) (Math|Rotator|MakeRotator 0.0 0.0 (Math|Float|Lerp (Variables|Default|GetClosedAngle) (Variables|Default|GetOpenAngle) _doortrack)) false false))))))

(event EventInteract
  ;[1 1 1] Open/close door animation
  (Utilities|FlowControl|FlipFlop
    (:A
      (Variables|Default|SetIsDoorOpen true)
      (bind _doortrack (Timeline|Timeline_0 Play)
        (:Update
          (Transformation|SetRelativeRotation (Variables|Default|GetPorte) (Math|Rotator|MakeRotator 0.0 0.0 (Math|Float|Lerp (Variables|Default|GetClosedAngle) (Variables|Default|GetOpenAngle) _doortrack)) false false))))
    (:B
      (Timeline|Timeline_0 Reverse))))

(fn ConstructionScript
  (|CallParentFunction))