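; BP_LockDoor_2 is an interactable door that swings open and closed when interacted with.
; Each interaction alternates through a FlipFlop, playing or reversing a timeline whose track interpolates the Porte component's yaw between a closed and an open angle.
; Despite the name, no lock check runs; an old player-controller key check is left disconnected.
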(event EventInteract
  ;[1 1 1] Open/close door animation
  (Utilities|FlowControl|FlipFlop
    (:A
      (bind _doortrack (Timeline|Timeline_0 Play)
        (:Update
          (Transformation|SetRelativeRotation (Variables|Default|GetPorte) (Math|Rotator|MakeRotator 0.0 0.0 (Math|Float|Lerp (Variables|Default|GetClosedAngle) (Variables|Default|GetOpenAngle) _doortrack)) false false))))
    (:B
      (Timeline|Timeline_0 Reverse))))

(fn ConstructionScript
  (|CallParentFunction))