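; Interactable locked door that opens and closes only when the player controller's HasKeyOLD check passes.
; With the key, the first interaction plays a one-time explosion sound, and each interaction flip-flops a timeline between play and reverse.
; The timeline lerps the Porte component's yaw between ClosedAngle and OpenAngle.
; Without the key, interacting just plays a collapse sound cue.
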(event EventInteract
  (if (Variables|/Game/Blueprint/BP_Player/BP_PlayerController.BP_PlayerController_C|GetHasKeyOLD (Variables|Default|GetAs%20BP%20Player%20Controller))
    (Utilities|FlowControl|Sequence
      (:then_0
        (Utilities|FlowControl|DoOnce false
          (:Completed
            (Audio|PlaySound2D "/Game/StarterContent/Audio/Explosion01.Explosion01" 1.0 1.0 0.0 0 0))))
      (:then_1
        ;[1 1 1] Open/close door animation
        (Utilities|FlowControl|FlipFlop
          (:A
            (bind _doortrack (Timeline|Timeline_0 Play)
              (:Update
                (Transformation|SetRelativeRotation (Variables|Default|GetPorte) (Math|Rotator|MakeRotator 0.0 0.0 (Math|Float|Lerp (Variables|Default|GetClosedAngle) (Variables|Default|GetOpenAngle) _doortrack)) false false))))
          (:B
            (Timeline|Timeline_0 Reverse)))))
    (else
      (Audio|PlaySound2D "/Game/StarterContent/Audio/Collapse_Cue.Collapse_Cue" 1.0 1.0 0.0 0 0))))

(fn ConstructionScript
  (|CallParentFunction))