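; Interactable key pickup that grants the player the key and relocates the Jumeaux creature.
; Interact sets HasKeyOLD on the player controller, calls OnGet and destroys all BP_Creature_Jumeaux actors.
; If LocationToAppear is valid, it spawns a new creature at that transform running BT_Creature, then the key destroys itself.
; A box overlap with BP_Player creates and removes the WBP_PressE prompt.
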(event OnComponentBeginOverlap(Box)
  (params (OverlappedComponent :type Primitive%20Component%20Object%20Reference) (OtherActor :type Actor%20Object%20Reference) (OtherComp :type Primitive%20Component%20Object%20Reference) (OtherBodyIndex :type Integer) (bFromSweep :type Boolean) (SweepResult :type Hit%20Result%20Structure%20%28by%20ref%29))
  (Utilities|Casting|CastToBP_Player OtherActor)
  (bind _returnvalue (UserInterface|CreateWidget "/Game/Blueprint/UI/WBP_PressE.WBP_PressE_C"))
  (UserInterface|Viewport|AddtoViewport _returnvalue 0))

(event OnComponentEndOverlap(Box)
  (params (OverlappedComponent :type Primitive%20Component%20Object%20Reference) (OtherActor :type Actor%20Object%20Reference) (OtherComp :type Primitive%20Component%20Object%20Reference) (OtherBodyIndex :type Integer))
  (Utilities|Casting|CastToBP_Player OtherActor)
  (Widget|RemovefromParent (stale OnComponentBeginOverlap(Box) _returnvalue)))

(event EventInteract
  (bind _location_to_appear (Variables|Default|GetLocation%20to%20appear))
  (Variables|/Game/Blueprint/BP_Player/BP_PlayerController.BP_PlayerController_C|SetHasKeyOLD (Variables|Default|GetAs%20BP%20Player%20Controller) true)
  (Default|CallOnGet)
  (bind _outactors (Actor|GetAllActorsOfClass "/Game/Blueprint/IA2/BP_Creature_Jumeaux.BP_Creature_Jumeaux_C"))
  (Actor|DestroyActor _outactors)
  (if (Utilities|IsValid (Variables|Default|GetLocation%20to%20appear))
    (AI|SpawnAIFromClass "/Game/Blueprint/IA2/BP_Creature_Jumeaux.BP_Creature_Jumeaux_C" "/Game/Blueprint/IA2/BT_Creature.BT_Creature" (Transformation|GetActorLocation _location_to_appear) (Transformation|GetActorRotation _location_to_appear) false 0))
  (Actor|DestroyActor))

(fn ConstructionScript
  (|CallParentFunction))