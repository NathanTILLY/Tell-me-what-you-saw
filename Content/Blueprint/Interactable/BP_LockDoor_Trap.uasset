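; Interactable trap door that opens only when the player controller holds a key, otherwise playing a locked sound.
; The first successful interaction plays an unlock sound, spawns a creature leader AI at a spawn point and calls the player controller's StunTrap.
; Each successful interaction also toggles the door through a FlipFlop, with a timeline lerping its yaw between closed and open angles.
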(event EventInteract
  (bind _porte (Variables|Default|GetPorte))
  (bind _spawn_location (Variables|Default|GetSpawn_Location))
  (bind _returnvalue (Transformation|GetWorldLocation _porte))
  (bind _rootcomponent (Variables|/Script/Engine.Actor|GetRootComponent _spawn_location))
  (if (Variables|/Game/Blueprint/BP_Player/BP_PlayerController.BP_PlayerController_C|GetHasKeyOLD (Variables|Default|GetAs%20BP%20Player%20Controller))
    (Utilities|FlowControl|Sequence
      (:then_0
        (Utilities|FlowControl|DoOnce false
          (:Completed
            (Audio|PlaySoundatLocation "/Game/Sound/Porte/Porte_Ouverte_clé1.Porte_Ouverte_clé1" (Transformation|GetWorldLocation (Variables|Default|GetPorte)) "0, 0, 0" 1.0 1.0 0.0 0 0 0)
            (AI|SpawnAIFromClass "/Game/Blueprint/IA2/BP_Creature_Leader.BP_Creature_Leader_C" "/Game/Blueprint/IA2/BT_Creature.BT_Creature" (Transformation|GetWorldLocation _rootcomponent) (Transformation|GetWorldRotation _rootcomponent) false 0)
            (bind _asbp_player_controller (Utilities|Casting|CastToBP_PlayerController (Game|GetPlayerController 0)))
            (Default|StunTrap _asbp_player_controller)
            (Audio|PlaySound2D 0 1.0 1.0 0.0 0 0))))
      (:then_1
        ;[1 1 1] Open/close door animation
        (Utilities|FlowControl|FlipFlop
          (:A
            (Audio|PlaySoundatLocation "/Game/Sound/Porte/Porte_Ouvre_1__1_.Porte_Ouvre_1__1_" _returnvalue "0, 0, 0" 1.0 1.0 0.0 0 0 0)
            (bind _doortrack (Timeline|Timeline_0 Play)
              (:Update
                (Transformation|SetRelativeRotation (Variables|Default|GetPorte) (Math|Rotator|MakeRotator 0.0 0.0 (Math|Float|Lerp (Variables|Default|GetClosedAngle) (Variables|Default|GetOpenAngle) _doortrack)) false false))))
          (:B
            (Audio|PlaySoundatLocation "/Game/Sound/Porte/Porte_Ouvre_2.Porte_Ouvre_2" _returnvalue "0, 0, 0" 1.0 1.0 0.0 0 0 0)
            (Timeline|Timeline_0 Reverse)))))
    (else
      (Audio|PlaySoundatLocation "/Game/Sound/Porte/PorteFerme_3.PorteFerme_3" (Transformation|GetWorldLocation (Variables|Default|GetPorte)) "0, 0, 0" 1.0 1.0 0.0 0 0 0))))

(fn ConstructionScript
  (|CallParentFunction))