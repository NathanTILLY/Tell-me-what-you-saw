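; BP_LockDoor_Rire is an interactable door that plays a one-time 2D sound when the player interacts without the key.
; Interact calls the parent behavior in both cases, branching on the player controller's HasKeyOLD flag.
; The keyless branch plays Starter_Birds01 and sets RireFait, but only if neither this door nor its linked OtherDoor has already set that flag, so the pair shares a single trigger.
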(event EventInteract
  (if (Variables|/Game/Blueprint/BP_Player/BP_PlayerController.BP_PlayerController_C|GetHasKeyOLD (Variables|Default|GetAs%20BP%20Player%20Controller))
    (|CallParentFunction)
    (else
      (|CallParentFunction)
      (if (not (or (Variables|BP_LockDoor_Rire_C|GetRireFait? (Variables|Default|GetOtherDoor)) (Variables|Default|GetRireFait?)))
        (Audio|PlaySound2D "/Game/StarterContent/Audio/Starter_Birds01.Starter_Birds01" 1.0 1.0 0.0 0 0)
        (Variables|Default|SetRireFait? true)))))

(fn ConstructionScript
  (|CallParentFunction))