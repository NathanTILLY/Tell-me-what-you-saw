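; BP_Trigger_narratif_box is a trigger that fires a one-time scripted event when the player enters it after taking enough meds.
; On overlap, it compares the MedocPris stat from BP_PlayerController against the MedocNeedToTrigger threshold.
; A DoOnce then pushes the referenced Object's mesh with a force, plays an explosion sound at its location, and turns on two linked lights through CheckLightState.
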(event Collision|EventActorBeginOverlap
  (params (OtherActor :type Actor%20Object%20Reference))
  (bind _light_2 (Variables|Default|GetLight_2))
  (bind _light_1 (Variables|Default|GetLight_1))
  (if (== OtherActor (Game|Player|GetPlayerPawn 0))
    (bind _asbp_player_controller (Utilities|Casting|CastToBP_PlayerController (Game|GetPlayerController 0)))
    (if (>= (Variables|/Game/Blueprint/BP_Player/BP_PlayerStats.BP_PlayerStats_C|GetMedocPris (Default|GetStats _asbp_player_controller)) (Variables|Default|GetMedoc%20need%20to%20trigger))
      (Utilities|FlowControl|DoOnce false
        (:Completed
          (Physics|AddForce (Variables|/Script/Engine.StaticMeshActor|GetStaticMeshComponent (Variables|Default|GetObject)) "0.000000,600000.000000,0.000000" "None" false)
          (Audio|PlaySoundatLocation "/Game/StarterContent/Audio/Explosion01.Explosion01" (Transformation|GetActorLocation (Variables|Default|GetObject)) "0, 0, 0" 1.0 1.0 0.0 0 0 0)
          (Variables|/Game/Blueprint/Light/BP_Light.BP_Light_C|SetVisible%20On _light_1 true)
          (Default|CheckLightState _light_1)
          (Variables|/Game/Blueprint/Light/BP_Light.BP_Light_C|SetVisible%20On _light_2 true)
          (Default|CheckLightState _light_2))))))

(fn ConstructionScript)