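; BP_Light is a rect light actor that can blink at random.
; BeginPlay sets the light's visibility from the VisibleOn flag.
; Tick runs the blink only while ClignoteOn equals VisibleOn, so it also runs when both are false.
; A latent random Delay of a few seconds throttles Tick, then visibility is set to a random boolean, so the state may stay unchanged.
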(event EventBeginPlay
  (Rendering|SetVisibility (Variables|Default|GetRectLight) (Variables|Default|GetVisible%20On) false))

(event EventTick
  (params (DeltaSeconds :type Float%20%28single-precision%29))
  (if (Math|Boolean|Equal(Boolean) (Variables|Default|GetClignote%20On) (Variables|Default|GetVisible%20On))
    (Utilities|FlowControl|Delay (Math|Random|RandomFloatinRange 2.0 4.0))
    (Rendering|SetVisibility (Variables|Default|GetRectLight) (Math|Random|RandomBool) false)))

(fn ConstructionScript)