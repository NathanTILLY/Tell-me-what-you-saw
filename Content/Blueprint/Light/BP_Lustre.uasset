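; BP_Lustre is a chandelier that can drop as a physics object and play an explosion sound on its first hit.
; At BeginPlay it binds an event to the OnGet of BP_InteractableKey, while Fall enables physics on its Sphere.
; The impact sound plays at the world origin.
; A timeline for light flicker, dimmed once physics starts, is present but never runs, as LightVariationChandelier is empty.
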(event OnComponentHit(Sphere)
  (params (HitComponent :type Primitive%20Component%20Object%20Reference) (OtherActor :type Actor%20Object%20Reference) (OtherComp :type Primitive%20Component%20Object%20Reference) (NormalImpulse :type Vector :default "0, 0, 0") (Hit :type Hit%20Result%20Structure%20%28by%20ref%29))
  (Utilities|FlowControl|DoOnce false
    (:Completed
      (Audio|PlaySoundatLocation "/Game/StarterContent/Audio/Explosion02.Explosion02" "0, 0, 0" "0, 0, 0" 1.0 1.0 0.0 0 0 0))))

(event Custom|Light%20variation%20chandelier)

(event Custom|Fall
  (Physics|SetSimulatePhysics (Variables|Default|GetSphere) true))

(event EventBeginPlay
  (CallFunction|LightVariationChandelier)
  (bind _returnvalue (Actor|GetActorOfClass "/Game/Blueprint/Interactable/BP_InteractableKey.BP_InteractableKey_C"))
  (EventDispatchers|BindEventtoOnGet _returnvalue (EventDispatchers|CreateEvent :!event Custom|Fall)))

(fn ConstructionScript)