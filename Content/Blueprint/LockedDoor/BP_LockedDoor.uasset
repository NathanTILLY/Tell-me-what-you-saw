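; BP_LockedDoor is a door meant to swing open and closed for a nearby player holding a key.
; Box overlap enables or disables player input and opens or closes a Gate.
; The Gate's exit feeds a FlipFlop that plays or reverses a timeline, lerping the door's yaw.
; The key check that enters the Gate has no triggering event, so nothing here drives the animation.
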(event OnComponentBeginOverlap(Box)
  (params (OverlappedComponent :type Primitive%20Component%20Object%20Reference) (OtherActor :type Actor%20Object%20Reference) (OtherComp :type Primitive%20Component%20Object%20Reference) (OtherBodyIndex :type Integer) (bFromSweep :type Boolean) (SweepResult :type Hit%20Result%20Structure%20%28by%20ref%29))
  ;[1 1 1] Open door if close enough and hasKey
  (bind _asbp_player_controller (Utilities|Casting|CastToBP_PlayerController OtherActor))
  (Input|EnableInput (Game|GetPlayerController 0) 0)
  (Utilities|FlowControl|Gate true) ; enters at Open
)

(event OnComponentEndOverlap(Box)
  (params (OverlappedComponent :type Primitive%20Component%20Object%20Reference) (OtherActor :type Actor%20Object%20Reference) (OtherComp :type Primitive%20Component%20Object%20Reference) (OtherBodyIndex :type Integer))
  ;[1 1 1] Open door if close enough and hasKey
  (Utilities|Casting|CastToBP_PlayerController OtherActor)
  (Input|DisableInput (Game|GetPlayerController 0))
  (Utilities|FlowControl|Gate true) ; enters at Close
)

(event Input|ActionEvents|InputActionInteract
  (params (Key :type Key%20Structure :default "None"))
  ;[1 1 1] Open door if close enough and hasKey
)

(fn ConstructionScript)