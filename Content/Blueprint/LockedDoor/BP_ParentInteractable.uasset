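; Base interactable Blueprint that lets the player trigger an interaction while inside its Box trigger.
; When BP_Player begins overlapping, it binds an event to the ONINTERACT dispatcher on BP_PlayerController.
; Leaving the box unbinds every listener on that dispatcher, including any bound by other objects.
; Interact only prints a placeholder asking for an override; no door or key logic is implemented here.
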(event OnComponentBeginOverlap(Box)
  (params (OverlappedComponent :type Primitive%20Component%20Object%20Reference) (OtherActor :type Actor%20Object%20Reference) (OtherComp :type Primitive%20Component%20Object%20Reference) (OtherBodyIndex :type Integer) (bFromSweep :type Boolean) (SweepResult :type Hit%20Result%20Structure%20%28by%20ref%29))
  (bind _returnvalue (Game|GetPlayerController 0))
  (bind _asbp_player_controller (Utilities|Casting|CastToBP_PlayerController _returnvalue))
  ;[1 1 1] Open door if close enough and hasKey
  (Utilities|Casting|CastToBP_Player OtherActor)
  (Variables|Default|SetAs%20BP%20Player%20Controller _asbp_player_controller)
  (EventDispatchers|AssignONINTERACT _asbp_player_controller (EventDispatchers|CreateEvent :!event Custom|Interact)))

(event OnComponentEndOverlap(Box)
  (params (OverlappedComponent :type Primitive%20Component%20Object%20Reference) (OtherActor :type Actor%20Object%20Reference) (OtherComp :type Primitive%20Component%20Object%20Reference) (OtherBodyIndex :type Integer))
  ;[1 1 1] Open door if close enough and hasKey
  (Utilities|Casting|CastToBP_Player OtherActor)
  (EventDispatchers|UnbindallEventsfromONINTERACT (.AsBP%20Player%20Controller (Utilities|Casting|CastToBP_PlayerController (Game|GetPlayerController 0)))))

(event Custom|Interact
  ;[1 1 1] Open door if close enough and hasKey
  (Development|PrintString "Default interact please override"))

(fn ConstructionScript)

(fn NewFunction0)