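; Locked door actor that the player can open and close only while holding a key.
; On Interact, it checks the HasKeyOLD flag on a stored BP player controller reference, which is not assigned in these graphs.
; A FlipFlop alternates between playing and reversing a timeline, whose track lerps the Porte component's yaw between the closed and open angles.
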(event EventBeginPlay)

(event Collision|EventActorBeginOverlap
  (params (OtherActor :type Actor%20Object%20Reference)))

(event EventTick
  (params (DeltaSeconds :type Float%20%28single-precision%29)))

(event EventInteract
  (if (Variables|/Game/Blueprint/BP_Player/BP_PlayerController.BP_PlayerController_C|GetHasKeyOLD (Variables|Default|GetAs%20BP%20Player%20Controller))
    ;[1 1 1] Open/close door animation
    (Utilities|FlowControl|FlipFlop
      (:A
        (bind _doortrack (Timeline|Timeline_0 Play)
          (:Update
            (Transformation|SetRelativeRotation (Variables|Default|GetPorte) (Math|Rotator|MakeRotator 0.0 0.0 (Math|Float|Lerp (Variables|Default|GetClosedAngle) (Variables|Default|GetOpenAngle) _doortrack)) false false))))
      (:B
        (Timeline|Timeline_0 Reverse)))))

(fn ConstructionScript
  (|CallParentFunction))